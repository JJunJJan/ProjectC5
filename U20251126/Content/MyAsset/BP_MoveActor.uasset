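; BP_MoveActor moves its StaticMesh component in a staircase path, alternating between the positive X and Y axes.
; Each Tick adds a fixed, frame-rate-dependent step to the relative location and prints the accumulated distance.
; When that distance in hundreds of units reaches PreCountX or PreCountY, it resets and IsXY flips the axis.
; The other EventGraph chains are unconnected movement and string-function experiments that never run.
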(event `self.ReceiveTick`
  (params (DeltaSeconds :type "Float (single-precision)"))
  (bind _distance (`self.distance`))
  (bind _returnvalue (/ _distance 100))
  (`|ExecutionSequence`
    (:`then_0`
      ; LocationX 에 더한값을  LocationX 에 넣는다
      (if (`self.IsXY`)
        (set `self.LocationX` (+ (`self.LocationX`) 10.0))
        (else
          (set `self.LocationY` (+ (`self.LocationY`) 10.0))))
      (set `self.distance` (+ (`self.distance`) 10.0))
      (`SceneComponent.K2_SetRelativeLocation` (`self.StaticMesh`) (`KismetMathLibrary.MakeVector` (`self.LocationX`) (`self.LocationY`)) false false)
      (`KismetSystemLibrary.PrintString` (`KismetStringLibrary.Concat_StrStr` "distance : " (`KismetStringLibrary.Conv_Int64ToString` (`KismetMathLibrary.Conv_DoubleToInt64` _distance)) " / " "num : " (`KismetStringLibrary.Conv_IntToString` _returnvalue)))
      (if (`self.IsXY`)
        (if (>= _returnvalue (`self.preCountX`))
          (set `self.distance` 0.0 :!label _label)
          (if (`self.IsXY`)
            (set `self.IsXY` false)
            (else
              (set `self.IsXY` true))))
        (elif (>= _returnvalue (`self.preCountY`))
          (goto _label))))))

(fn `UserConstructionScript`)